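; Base player character for a game with a view that rotates in 90-degree steps, handling movement, jump, attack and ability unlocks.
; Rotate inputs update the shared GMRule angle, turn the spring arm and recompute movement vectors.
; Each tick, velocity along the active axis snaps control rotation to face travel direction.
; Attack plays a slot animation override tracking IsAttacking; its overlap only casts to monsters, and GainAbility enables double jump.
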(event `self.ReceiveBeginPlay`
  (`parent.ReceiveBeginPlay`)
  (`self.EnableAttackCollision` false)
  (set `self.Faction` "NewEnumerator0"))

(event `self.ReceiveTick`
  (params (DeltaSeconds :type "Float (single-precision)"))
  (`parent.ReceiveTick` 0.0)
  (`self.UpdateControllerRotation`))

(event `InputAxis|Move_Y`
  (params (AxisValue :type "Float (single-precision)"))
  (if (`self.CanAct`)
    (`self.AddMovementInput` (* (`self.Move_Y_Vector`) AxisValue))))

(event `InputAxis|Move_X`
  (params (AxisValue :type "Float (single-precision)"))
  (if (`self.CanAct`)
    (`self.AddMovementInput` (* (`self.Move_X_Vector`) AxisValue))))

(event `InputAction|Jump`
  (params (Key :type "Key Structure"))
  (:`Pressed`
    (if (`self.CanAct`)
      (`self.Jump`)))
  (:`Released`
    (`self.StopJumping`)))

(event `InputAction|Attack`
  (params (Key :type "Key Structure"))
  (:`Pressed`
    (if (`self.CanAct`)
      (`PaperZDPlaySlotOverrideAction.PlayAnimationOverrideWithCallbacks` (`self.GetAnimInstance`) "/Game/BluePrints/Characters/Player/Captain/AnimSequences/Attack.Attack" "AttackSlot"
        (:`then`
          (set `self.IsAttacking` true))
        (:`OnCompleted`
          (set `self.IsAttacking` false :!label _label))
        (:`OnCancelled`
          (goto _label))))))

(event `self.AttackCollision.OnComponentBeginOverlap`
  (params (OverlappedComponent :type "PrimitiveComponent Object Reference") (OtherActor :type "Actor Object Reference") (OtherComp :type "PrimitiveComponent Object Reference") (OtherBodyIndex :type Integer) (bFromSweep :type Boolean) (SweepResult :type "HitResult Structure (by ref)"))
  (cast `/Game/BluePrints/Characters/Monsters/BP_Character_Monster_Base` OtherActor))

(event `InputAction|RotateRight`
  (params (Key :type "Key Structure"))
  (:`Pressed`
    (`self.WorldRotation` -90.0)))

(event `InputAction|RotateLeft`
  (params (Key :type "Key Structure"))
  (:`Pressed`
    (`self.WorldRotation` 90.0)))

(fn `GainAbility`
  (params (UnlockAbility :type "/Game/BluePrints/Enums/E_Abilities Enum (by ref)"))
  (`KismetArrayLibrary.Array_AddUnique` (`self.UnlockedAbilities`) UnlockAbility)
  (switch `/Game/BluePrints/Enums/E_Abilities` (`local.UnlockAbility`)
    (:`NewEnumerator0`
      (set `self.JumpMaxCount` 2))))

(fn `UpdateControllerRotation`
  (bind _returnvalue (`self.GetController`))
  (bind _returnvalue_2 (`self.GetController`))
  (bind _returnvalue_3 (`self.GetController`))
  (bind _returnvalue_4 (`self.GetController`))
  (bind (_velocity_x _velocity_y) (`KismetMathLibrary.BreakVector` (`MovementComponent.Velocity` (`self.CharacterMovement`))))
  (bind _velocity_x_2 (`KismetMathLibrary.BreakVector` (`MovementComponent.Velocity` (`self.CharacterMovement`))))
  (if (== (mod (/ (`/Game/BluePrints/GameMode/GM_MainRule.RotationAngle` (`self.GMRule`)) 90.0) 2.0) 0.0)
    (`/Engine/EditorBlueprintResources/StandardMacros.CompareFloat` _velocity_x_2
      (:`>`
        (`/Engine/EditorBlueprintResources/StandardMacros.IsValid` _returnvalue_2
          (:`Is Valid`
            (`Controller.SetControlRotation` _returnvalue_2 (`KismetMathLibrary.MakeRotator` 0.0)))))
      (:`<`
        (`/Engine/EditorBlueprintResources/StandardMacros.IsValid` _returnvalue_3
          (:`Is Valid`
            (`Controller.SetControlRotation` _returnvalue_3 (`KismetMathLibrary.MakeRotator` 0.0 0.0 (+ 0.0 180.0)))))))
    (else
      (`/Engine/EditorBlueprintResources/StandardMacros.CompareFloat` _velocity_y
        (:`>`
          (`/Engine/EditorBlueprintResources/StandardMacros.IsValid` _returnvalue_4
            (:`Is Valid`
              (`Controller.SetControlRotation` _returnvalue_4 (`KismetMathLibrary.MakeRotator` 0.0 0.0 90.0)))))
        (:`<`
          (`/Engine/EditorBlueprintResources/StandardMacros.IsValid` _returnvalue
            (:`Is Valid`
              (`Controller.SetControlRotation` _returnvalue (`KismetMathLibrary.MakeRotator` 0.0 0.0 (+ 90.0 180.0))))))))))

(fn `UserConstructionScript`
  (`parent.UserConstructionScript`))

(fn `WorldRotation`
  (params (RotationAngle :type "Float (double-precision)"))
  (bind (_returnvalue_roll _returnvalue_pitch _returnvalue_yaw) (`KismetMathLibrary.BreakRotator` (`SceneComponent.K2_GetComponentRotation` (`self.SpringArm`))))
  (set `/Game/BluePrints/GameMode/GM_MainRule.RotationAngle` (mod (+ (`/Game/BluePrints/GameMode/GM_MainRule.RotationAngle` (`self.GMRule`)) RotationAngle) 360.0) (`self.GMRule`))
  (`self.UpdateControllerRotation`)
  (`SceneComponent.K2_SetWorldRotation` (`self.SpringArm`) (`KismetMathLibrary.MakeRotator` _returnvalue_roll _returnvalue_pitch (+ (`local.RotationAngle`) _returnvalue_yaw)) false false)
  (bind _output_get (set `self.MoveXRotator` (`KismetMathLibrary.MakeRotator` 0.0 0.0 (`/Game/BluePrints/GameMode/GM_MainRule.RotationAngle` (`self.GMRule`)))))
  (set `self.Move_X_Vector` (`KismetMathLibrary.GetForwardVector` _output_get))
  (bind _output_get_2 (set `self.MoveYRotator` (`KismetMathLibrary.MakeRotator` 0.0 0.0 (+ (`/Game/BluePrints/GameMode/GM_MainRule.RotationAngle` (`self.GMRule`)) 90.0))))
  (set `self.Move_Y_Vector` (`KismetMathLibrary.GetForwardVector` _output_get_2))
  (set `/Game/BluePrints/GameMode/GM_MainRule.NowDirection` (`self.Move_X_Vector`) (`self.GMRule`)))