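; BP_Sworld is a sword actor for the Captain player character, with a flipbook sprite and a Box collider.
; Overlapping a BP_Character_Monster_Base deals fixed damage through ReceiveAttact and destroys the sword.
; A Box hit switches the sprite to the non-looping idle flipbook, reduces the box's Z extent and makes it block Pawns, leaving a solid resting sword.
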(event `self.Box.OnComponentHit`
  (params (HitComponent :type "PrimitiveComponent Object Reference") (OtherActor :type "Actor Object Reference") (OtherComp :type "PrimitiveComponent Object Reference") (NormalImpulse :type "Vector Structure") (Hit :type "HitResult Structure (by ref)"))
  (bind (_boxextent_x _boxextent_y _boxextent_z) (`KismetMathLibrary.BreakVector` (`BoxComponent.BoxExtent` (`self.Box`))))
  (`PaperFlipbookComponent.SetFlipbook` (`self.Sword`) "/Game/Assets/Sword/Captain__Sword_Idle.Captain__Sword_Idle")
  (`PaperFlipbookComponent.SetLooping` (`self.Sword`) false)
  (`BoxComponent.SetBoxExtent` (`self.Box`) (`KismetMathLibrary.MakeVector` _boxextent_x _boxextent_y (- _boxextent_z 16.0)) true)
  (`PrimitiveComponent.SetCollisionResponseToChannel` (`self.Box`) "ECC_Pawn" "ECR_Block"))

(event `self.Box.OnComponentBeginOverlap`
  (params (OverlappedComponent :type "PrimitiveComponent Object Reference") (OtherActor :type "Actor Object Reference") (OtherComp :type "PrimitiveComponent Object Reference") (OtherBodyIndex :type Integer) (bFromSweep :type Boolean) (SweepResult :type "HitResult Structure (by ref)"))
  (bind _asbp_character_monster_base (cast `/Game/BluePrints/Characters/Monsters/BP_Character_Monster_Base` OtherActor))
  (`/Game/BluePrints/Characters/BP_Character_base.ReceiveAttact` _asbp_character_monster_base 20.0)
  (`self.K2_DestroyActor`))

(fn `UserConstructionScript`)