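; Base Blueprint for sprite-based combat characters, handling health, melee hits between factions, stun and defeat.
; A toggleable attack collision damages opposing-faction characters and applies hit stop to both sides by briefly zeroing CustomTimeDilation.
; Taking a hit plays a sound, then either stuns with a timer-driven sprite shake or triggers defeat, which disables capsule collision and starts a removal timer.
; Animation changes use JumpToNode, and CanAct blocks action while attacking, stunned or defeated.
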(event `self.ReceiveBeginPlay`
  (set `self.Health` (`self.Maxhealth`))
  (set `self.SpriteRelativeLocation` (`SceneComponent.RelativeLocation` (`self.Sprite`)))
  (`PrimitiveComponent.SetCollisionEnabled` (`self.AttackCollision`) "NoCollision"))

(event `self.ReceiveTick`
  (params (DeltaSeconds :type "Float (single-precision)"))
  (`parent.ReceiveTick` 0.0))

(event `self.AttackCollision.OnComponentBeginOverlap`
  (params (OverlappedComponent :type "PrimitiveComponent Object Reference") (OtherActor :type "Actor Object Reference") (OtherComp :type "PrimitiveComponent Object Reference") (OtherBodyIndex :type Integer) (bFromSweep :type Boolean) (SweepResult :type "HitResult Structure (by ref)"))
  (bind _asbp_character_base (cast `/Game/BluePrints/Characters/BP_Character_base` OtherActor))
  (if (`|EnumInequality` (`/Game/BluePrints/Characters/BP_Character_base.Faction` _asbp_character_base) (`self.Faction`))
    (`self.ReceiveAttact` _asbp_character_base (`self.AttackDamage`))
    (`self.HitStop` _asbp_character_base (`self.AttackStopDuration`))
    (`self.HitStop` (`self.SelfAttackStopDuration`))))

(event `HitStop`
  (params (StopDuration :type "Float (double-precision)"))
  (set `self.CustomTimeDilation` 0.0)
  (`KismetSystemLibrary.RetriggerableDelay` StopDuration)
  (set `self.CustomTimeDilation` 1.0))

(event `ShakeCharacter`
  (bind (_spriterelativelocation_x _spriterelativelocation_y _spriterelativelocation_z) (`KismetMathLibrary.BreakVector` (`self.SpriteRelativeLocation`)))
  (bind _isa (`/Engine/EditorBlueprintResources/StandardMacros.FlipFlop`)
    (:`A`
      _)
    (:`B`
      _))
  (`SceneComponent.K2_SetRelativeLocation` (`self.Sprite`) (`KismetMathLibrary.MakeVector` (+ _spriterelativelocation_x (`KismetMathLibrary.SelectFloat` 5.0 -5.0 _isa)) _spriterelativelocation_y _spriterelativelocation_z) false false))

(fn `CanAct`
  (returns (CanAct :type Boolean))
  (return (not (or (`self.IsAttacking`) (`self.IsStun`) (`self.IsDefeated`)))))

(fn `ClearSelf`
  (`self.K2_DestroyActor`))

(fn `ClearStun`
  (bind _output_get (set `self.IsStun` false))
  (`self.StunStateChange` _output_get)
  (`KismetSystemLibrary.K2_ClearAndInvalidateTimerHandle` (`self.StunShake`))
  (`SceneComponent.K2_SetRelativeLocation` (`self.Sprite`) (`self.SpriteRelativeLocation`) false false))

(fn `EnableAttackCollision`
  (params (IsActive :type Boolean))
  (bind _attackcollision (`self.AttackCollision`))
  (if IsActive
    (`PrimitiveComponent.SetCollisionEnabled` _attackcollision "QueryOnly")
    (else
      (`PrimitiveComponent.SetCollisionEnabled` _attackcollision "NoCollision"))))

(fn `ReceiveAttact`
  (params (Damage :type "Float (double-precision)"))
  (`GameplayStatics.PlaySoundAtLocation` "/Game/Assets/Action_Platformer_Sounds/S_Hit_Cue.S_Hit_Cue" (`self.K2_GetActorLocation`) (struct) 1.0 1.0 0.0 null null null)
  (if (not (`self.IsDefeated`))
    (set `self.Health` (- (`self.Health`) (`local.Damage`)))
    (`PaperZDAnimInstance.StopAllAnimationOverrides` (`self.GetAnimInstance`))
    (if (> (`self.Health`) 0.0)
      (bind _output_get (set `self.IsStun` true))
      (`self.StunStateChange` _output_get)
      (`PaperZDAnimInstance.JumpToNode` (`self.GetAnimInstance`) "Stun_Jump" "None")
      (`KismetSystemLibrary.K2_SetTimerDelegate` (`|CreateDelegate` :!event `ClearStun`) 0.5)
      (bind _returnvalue (`KismetSystemLibrary.K2_SetTimerDelegate` (`|CreateDelegate` :!event `ShakeCharacter`) 0.055 true))
      (set `self.StunShake` _returnvalue)
      (else
        (set `self.IsDefeated` true :!label _label)
        (`PaperZDAnimInstance.JumpToNode` (`self.GetAnimInstance`) "DefeatJump" "None")
        (`PrimitiveComponent.SetCollisionEnabled` (`self.CapsuleComponent`) "NoCollision")
        (`KismetSystemLibrary.K2_SetTimerDelegate` (`|CreateDelegate` :!event `ClearSelf`) 10.0)))
    (else
      (goto _label))))

(fn `UserConstructionScript`)