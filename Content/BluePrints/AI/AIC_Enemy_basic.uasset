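; AI controller for basic enemies that runs the enemy behavior tree and tracks the player pawn as its attack target.
; On possession it binds to the monster's stun event and mirrors that state into the blackboard.
; Each tick it points focus toward the target, scaled by the absolute game-mode direction vector, or straight ahead when the monster cannot act.
; A separate function writes an attack target to the blackboard.
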(event `self.ReceiveBeginPlay`
  (`self.UseBlackboard` "/Game/BluePrints/AI/BB_Enemy.BB_Enemy")
  (`self.RunBehaviorTree` "/Game/BluePrints/AI/BT_Enemy.BT_Enemy")
  (bind _asbp_character_player_base (cast `/Game/BluePrints/Characters/Player/BP_Character_Player_Base` (`GameplayStatics.GetPlayerPawn` 0)))
  (set `self.AttackTarget` _asbp_character_player_base)
  (bind _asgm_main_rule (cast `/Game/BluePrints/GameMode/GM_MainRule` (`GameplayStatics.GetGameMode`)))
  (set `self.GMRule` _asgm_main_rule))

(event `self.ReceiveTick`
  (params (DeltaSeconds :type "Float (single-precision)"))
  (`self.SetFocusDirection`))

(event `self.ReceivePossess`
  (params (PossessedPawn :type "Pawn Object Reference"))
  (bind _asbp_character_monster_base (cast `/Game/BluePrints/Characters/Monsters/BP_Character_Monster_Base` PossessedPawn))
  (bind _output_get (set `self.PossesedMonsterBase` _asbp_character_monster_base))
  (add `/Game/BluePrints/Characters/BP_Character_base.StunStateChange` _output_get (delegate `OnStunStateChange`)))

(event `OnStunStateChange`
  (params (Stuned :type Boolean))
  (`BlackboardComponent.SetValueAsBool` (`self.Blackboard`) (`self.isStunKey`) Stuned))

(fn `SetAttackTarget`
  (params (Attacktarget :type "/Game/BluePrints/Characters/Player/BP_Character_Player_Base Object Reference"))
  (`BlackboardComponent.SetValueAsObject` (`self.Blackboard`) (`self.AttacktargetKeyName`) (`local.Attacktarget`)))

(fn `SetFocusDirection`
  (bind _possesedmonsterbase (`self.PossesedMonsterBase`))
  (`/Engine/EditorBlueprintResources/StandardMacros.IsValid` (`self.AttackTarget`)
    (:`Is Valid`
      (if (`/Game/BluePrints/Characters/BP_Character_base.CanAct` (`self.PossesedMonsterBase`))
        (if true
          (`self.K2_SetFocalPoint` (+ (`self.K2_GetActorLocation` (`self.PossesedMonsterBase`)) (* (`KismetMathLibrary.GetForwardVector` (`KismetMathLibrary.FindLookAtRotation` (`self.K2_GetActorLocation` (`self.PossesedMonsterBase`)) (`self.K2_GetActorLocation` (`self.AttackTarget`)))) (`KismetMathLibrary.Vector_GetAbs` (`/Game/BluePrints/GameMode/GM_MainRule.NowDirection` (`self.GMRule`)))))))
        (else
          (`self.K2_SetFocalPoint` (+ (`self.GetActorForwardVector` _possesedmonsterbase) (`self.K2_GetActorLocation` _possesedmonsterbase))))))))

(fn `UserConstructionScript`)